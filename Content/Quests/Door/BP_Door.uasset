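; Door actor that opens and closes on a toggle event and can display a "Press E" prompt.
; ToggleDoor alternates playing and reversing the OpenDoor timeline, whose output drives the yaw of the SMDoor mesh.
; ShowPressE and HidePressE switch the prompt's visibility, which starts hidden from the construction script.
; Tick rotates the prompt every frame to face the player camera.
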(event `ToggleDoor`
  ; Toggle Door
  (`/Engine/EditorBlueprintResources/StandardMacros.FlipFlop`
    (:`A`
      (bind (_direction _z) (`Timeline|OpenDoor` :!label _label)
        (:`Update`
          (`SceneComponent.K2_SetRelativeRotation` (`self.SM_Door`) (`KismetMathLibrary.MakeRotator` 0.0 0.0 _z) false false))))
    (:`B`
      (goto _label :!via `Reverse`))))

(event `ShowPressE`
  ; Show/Hide Press E
  (`SceneComponent.SetVisibility` (`self.PressE`) true false))

(event `self.ReceiveTick`
  (params (DeltaSeconds :type "Float (single-precision)"))
  ; Press E look at the camera
  (`SceneComponent.K2_SetWorldRotation` (`self.PressE`) (`KismetMathLibrary.FindLookAtRotation` (`SceneComponent.K2_GetComponentLocation` (`self.PressE`)) (`self.K2_GetActorLocation` (`GameplayStatics.GetPlayerCameraManager` 0))) false false))

(event `HidePressE`
  ; Show/Hide Press E
  (`SceneComponent.SetVisibility` (`self.PressE`) false false))

(fn `UserConstructionScript`
  (`self.HidePressE`))