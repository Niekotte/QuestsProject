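; Player character Blueprint that interacts with doors, can switch possession to a BP_Player, and takes elemental damage.
; Each tick a forward line trace from the capsule caches the hit actor, driving the door's Press E prompt.
; IA_Interact reuses that hit to toggle doors or possess the BP_Player.
; Water, fire and poison events print debug text and reduce HP; a dot/cross-product backstab check is disabled.
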(event `LineForDoor`
  ; Door
  (if (`self.LineReturnValue`)
    (bind _asbp_door (cast `/Game/Quests/Door/BP_Door` (`self.A_HitActorValueLine`)))
    (`/Game/Quests/Door/BP_Door.ShowPressE` _asbp_door)
    (else
      (`/Engine/EditorBlueprintResources/StandardMacros.IsValid` _asbp_door
        (:`Is Valid`
          (`/Game/Quests/Door/BP_Door.HidePressE` _asbp_door))))))

(event `Line`
  (bind _capsulecomponent (`self.CapsuleComponent`))
  (bind _returnvalue (`SceneComponent.K2_GetComponentLocation` _capsulecomponent))
  ; Line
  (bind (_outhit _returnvalue_2) (`KismetSystemLibrary.LineTraceSingle` _returnvalue (+ _returnvalue (* (`SceneComponent.GetForwardVector` _capsulecomponent) 300.0)) "TraceTypeQuery1"))
  (set `self.LineReturnValue` _returnvalue_2)
  (set `self.A_HitActorValueLine` (`.HitActor` (`GameplayStatics.BreakHitResult` _outhit)))
  (`|ExecutionSequence`
    (:`then_0`
      (`self.LineForDoor`))
    (:`then_1`
      (`self.LineForBackstab` :!enabledstate Disabled))))

(event `EnhancedInput|/Game/Hub/Core/Input/Actions/IA_Interact`
  (params (ActionValue :type Boolean) (ElapsedSeconds :type "Float (double-precision)") (TriggeredSeconds :type "Float (double-precision)") (InputAction :type "InputAction Object Reference" :default "/Game/Hub/Core/Input/Actions/IA_Interact.IA_Interact"))
  ; Interact
  (:`Started`
    (if (`self.LineReturnValue`)
      (`|ExecutionSequence`
        (:`then_0`
          (bind _asbp_door (cast `/Game/Quests/Door/BP_Door` (`self.A_HitActorValueLine`)))
          (`/Game/Quests/Door/BP_Door.ToggleDoor` _asbp_door))
        (:`then_1`
          (bind _asbp_player (cast `/Game/Hub/Core/BP_Player` (`self.A_HitActorValueLine`)))
          (`KismetSystemLibrary.PrintString` "Miaou")
          (`Controller.Possess` (`GameplayStatics.GetPlayerController` 0) _asbp_player))))))

(event `self.ReceiveTick`
  (params (DeltaSeconds :type "Float (single-precision)"))
  ; Line
  (`self.Line`))

(event `self.EffetEau`
  ; Effects
  (`KismetSystemLibrary.PrintString` "Eau" true true (struct :`G` 0.044416 :`B` 1.0 :`A` 1.0))
  (`self.UpdateHP` -20.0))

(event `self.EffetFeu`
  ; Effects
  (`KismetSystemLibrary.PrintString` "Feu" true true (struct :`R` 1.0 :`G` 0.030687 :`B` 0.000118 :`A` 1.0))
  (`self.UpdateHP` -5.0))

(event `self.EffetPoison`
  ; Effects
  (`KismetSystemLibrary.PrintString` "Poison" true true (struct :`R` 1.0 :`B` 0.863157 :`A` 1.0))
  (`self.UpdateHP` -2.0))

(fn `UserConstructionScript`
  (`parent.UserConstructionScript`))